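; Player-drivable car Blueprint that takes hits, explodes and respawns at its starting transform.
; Forward and Right axis inputs drive the vehicle movement's throttle and steering; BeginPlay adds a HUD and caches the spawn transform.
; Each Shot removes one health and updates HealthPercentage, calling Kill at zero or below.
; Kill spawns explosion effects and a radially shattered DestructibleCube, then teleports the same car back with full health instead of destroying it.
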(event `Shot`
  (params (VehicleID :type Integer))
  (bind _result (`/Engine/EditorBlueprintResources/StandardMacros.DecrementInt` (stale `self.ReceiveBeginPlay` _output_get_2))
    (:`  `
      (set `self.healthPercentage` (/ (`KismetMathLibrary.Conv_IntToDouble` _result) (`KismetMathLibrary.Conv_IntToDouble` (`self.maxHealth`))))
      (`/Engine/EditorBlueprintResources/StandardMacros.CompareInt` _result
        (:`==`
          _)
        (:`<`
          _))
      (`self.Kill`))))

(event `Kill`
  (bind _returnvalue (`self.K2_GetActorLocation`))
  (bind _mesh (`self.Mesh`))
  ;[1 1 1] Death
  (`/Game/TurretAI/TargetCom.SetisDead` (`self.TargetCom`) true)
  (`GameplayStatics.SpawnEmitterAtLocation` "/Game/StarterContent/Particles/P_Explosion.P_Explosion" _returnvalue)
  (`GameplayStatics.PlaySoundAtLocation` "/Game/StarterContent/Audio/Explosion02.Explosion02" _returnvalue)
  (bind _returnvalue_2 (`|SpawnActorFromClass` "/Game/Destruction/destructibleCube.destructibleCube_C" (`KismetMathLibrary.Conv_VectorToTransform` _returnvalue) "AlwaysSpawn" "OverrideRootScale"))
  (`DestructibleComponent.ApplyRadiusDamage` (`/Game/Destruction/destructibleCube.Destructible` _returnvalue_2) 10000.0 _returnvalue 1000.0 1000.0 true)
  ;[1 1 1] Respawning
  (`PrimitiveComponent.SetPhysicsLinearVelocity` _mesh (0.0 0.0 0.0) false "None")
  (`SceneComponent.K2_SetWorldRotation` _mesh (`self.spawnRotation`) false false)
  (`SceneComponent.K2_SetWorldLocation` _mesh (`self.spawnLocation`) false true)
  (`/Game/TurretAI/TargetCom.SetisDead` (`self.TargetCom`) false)
  (set `self.currentHealth` (`self.maxHealth`))
  (set `self.healthPercentage` 1.0))

(event `self.ReceiveBeginPlay`
  (bind _mesh (`self.Mesh`))
  (bind _returnvalue (`|CreateWidget` "/Game/GUI/HUD.HUD_C"))
  (bind _output_get (set `self.HUD Reference` _returnvalue))
  (`UserWidget.AddToViewport` _output_get 0)
  (set `self.spawnLocation` (`SceneComponent.K2_GetComponentLocation` _mesh))
  (set `self.spawnRotation` (`SceneComponent.K2_GetComponentRotation` _mesh))
  (bind _output_get_2 (set `self.currentHealth` (`self.maxHealth`))))

(event `InputAxis|Forward`
  (params (AxisValue :type "Float (single-precision)"))
  ;[1 1 1] Driving
  (`WheeledVehicleMovementComponent.SetThrottleInput` (`self.VehicleMovement`) AxisValue))

(event `InputAxis|Right`
  (params (AxisValue :type "Float (single-precision)"))
  ;[1 1 1] Driving
  (`WheeledVehicleMovementComponent.SetSteeringInput` (`self.VehicleMovement`) AxisValue))

(fn `UserConstructionScript`)