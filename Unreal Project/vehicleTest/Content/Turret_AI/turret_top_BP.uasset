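; Player-controlled turret top that tilts with vertical mouse movement within a clamp angle and fires explosive hitscan shots.
; The Possessed event applies rotation and, while left mouse or right trigger is held, fires timed camera line traces with sound and explosion effects.
; Hits, detected by a nonzero coordinate sum, damage destructibles or call Shot on swan and AI cars.
; AI car hits add score, plus a low-health kill bonus; BeginPlay creates the HUD.
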(event `Key|LeftMouseButton`
  (params (Key :type "Key Structure" :default "AnyKey"))
  ;[1 1 1] Toggle whether left mouse button is held down or not
  (:`Pressed`
    (set `self.isPressed` true :!label _label))
  (:`Released`
    (set `self.isPressed` false :!label _label_2)))

(event `Key|Gamepad_RightTrigger`
  (params (Key :type "Key Structure" :default "AnyKey"))
  ;[1 1 1] Toggle whether left mouse button is held down or not
  (:`Pressed`
    (goto _label))
  (:`Released`
    (goto _label_2)))

(event `self.ReceiveBeginPlay`
  ;[1 1 1] Initialize variables
  (set `self.tickTime` 0.2)
  (set `self.deltaTime` 0.0)
  (set `self.isPressed` false)
  (set `self.ClampAngle` 45.0)
  (bind _returnvalue (`|CreateWidget` "/Game/GUI/HUD.HUD_C"))
  (bind _output_get (set `self.HUD Reference` _returnvalue))
  (`UserWidget.AddToViewport` _output_get 0))

(event `self.ReceivePossessed`
  (params (NewController :type "Controller Object Reference"))
  (bind _returnvalue (`GameplayStatics.GetPlayerController` 0))
  (bind _deltatime (`self.deltaTime`))
  (bind _camera (`self.Camera`))
  (bind (_deltax _deltay) (`PlayerController.GetInputMouseDelta` _returnvalue))
  (bind _returnvalue_2 (`SceneComponent.K2_GetComponentLocation` _camera))
  ;[1 1 1] Add rotation to the turret
  (if (`KismetSystemLibrary.IsValid` _returnvalue)
    (set `self.YRot` _deltay)
    (`/Engine/EditorBlueprintResources/StandardMacros.CompareFloat` (`KismetMathLibrary.Abs` (+ (.roll (`self.K2_GetActorRotation`)) (`self.YRot`))) (`self.ClampAngle`)
      (:`>`
        _)
      (:`==`
        (`SceneComponent.K2_AddRelativeRotation` (`self.turret_top`) (`KismetMathLibrary.MakeRotator` _deltay) false false :!label _label_3))
      (:`<`
        (goto _label_3)))
    ;[1 1 1] Do a line trace from the turret to 10000cm forward from the turret 5 times per second while shooting
    (set `self.deltaTime` (+ _deltatime (`GameplayStatics.GetWorldDeltaSeconds`)))
    (if (`self.isPressed`)
      (`/Engine/EditorBlueprintResources/StandardMacros.CompareFloat` _deltatime (`self.tickTime`)
        (:`>`
          _)
        (:`==`
          _))
      (set `self.deltaTime` 0.0)
      (`GameplayStatics.PlaySoundAtLocation` "/Game/Turret_AI/gunshot_Cue.gunshot_Cue" _returnvalue_2)
      (bind _outhit (`KismetSystemLibrary.LineTraceSingle` _returnvalue_2 (+ _returnvalue_2 (* (`KismetMathLibrary.RotateAngleAxis` (`SceneComponent.GetForwardVector` _camera) 0.0 (`SceneComponent.GetUpVector` _camera)) 10000.0)) "TraceTypeQuery1"))
      (bind (_bblockinghit _binitialoverlap _time _location _impactpoint _normal _impactnormal _physmat _hitactor) (`GameplayStatics.BreakHitResult` _outhit))
      ;[1 1 1] Get hit result from line trace and try casting it to various targets
      (`/Engine/EditorBlueprintResources/StandardMacros.CompareFloat` (+ (.x _location) (.y _location) (.z _location))
        (:`>`
          _)
        (:`<`
          _))
      (`GameplayStatics.SpawnEmitterAtLocation` "/Game/StarterContent/Particles/P_Explosion.P_Explosion" _location)
      (`GameplayStatics.PlaySoundAtLocation` "/Game/StarterContent/Audio/Explosion_Cue.Explosion_Cue" _location)
      (bind _asdestructible_actor (cast `DestructibleActor` _hitactor)
        (:`then`
          (`DestructibleComponent.ApplyRadiusDamage` (`DestructibleActor.DestructibleComponent` _asdestructible_actor) 1000.0 _location 1000.0 1000.0 false))
        (:`CastFailed`
          (bind _asswan_car_bp (cast `/Game/SwanCar/swanCarBP` _hitactor)
            (:`then`
              (`/Game/SwanCar/swanCarBP.Shot` _asswan_car_bp 0))
            (:`CastFailed`
              (bind _asaicar (cast `/Game/DefaultCar_AI/AICar` _hitactor))
              (`/Game/DefaultCar_AI/AICar.Shot` _asaicar 0)
              (`self.IncreaseScore` _asaicar))))))))

(fn `IncreaseScore`
  (params (AIActor :type "/Game/DefaultCar_AI/AICar Object Reference"))
  (bind _playerscore (`self.PlayerScore`))
  ;[1 1 1] Adding Score to Player
  (`/Engine/EditorBlueprintResources/StandardMacros.IncrementInt` _playerscore
    (:`  `
      (if (<= (`/Game/DefaultCar_AI/AICar.AI Health` AIActor) 1)
        (set `self.PlayerScore` (+ _playerscore (`self.KillValue`))))
      (`self.UpdatePlayerScore`))))

(fn `UserConstructionScript`)