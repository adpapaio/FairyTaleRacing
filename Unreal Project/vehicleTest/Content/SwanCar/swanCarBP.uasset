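; SwanCarBP is a shootable swan car that explodes when its health runs out.
; Health is set on BeginPlay, and each Shot event decrements it without using the VehicleID input.
; At zero or below, it flags TargetCom as dead, destroys itself, and spawns explosion particles and sound.
; It also spawns a DestructibleCube in its place and immediately shatters it with radius damage.
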(event `Shot`
  (params (VehicleID :type Integer))
  (bind _returnvalue (`self.K2_GetActorLocation`))
  (bind _result (`/Engine/EditorBlueprintResources/StandardMacros.DecrementInt` (stale `self.ReceiveBeginPlay` _output_get))
    (:`  `
      (`/Engine/EditorBlueprintResources/StandardMacros.CompareInt` _result
        (:`==`
          _)
        (:`<`
          _))
      (`/Game/Turret_AI/TargetCom.SetisDead` (`self.TargetCom`) true)
      (`self.K2_DestroyActor`)
      (`GameplayStatics.SpawnEmitterAtLocation` "/Game/StarterContent/Particles/P_Explosion.P_Explosion" _returnvalue)
      (`GameplayStatics.PlaySoundAtLocation` "/Game/StarterContent/Audio/Explosion02.Explosion02" _returnvalue)
      (bind _returnvalue_2 (`|SpawnActorFromClass` "/Game/Destruction/destructibleCube.destructibleCube_C" (`KismetMathLibrary.Conv_VectorToTransform` _returnvalue) "AlwaysSpawn" "OverrideRootScale"))
      (`DestructibleComponent.ApplyRadiusDamage` (`/Game/Destruction/destructibleCube.Destructible` _returnvalue_2) 10000.0 _returnvalue 1000.0 1000.0 true))))

(event `self.ReceiveBeginPlay`
  (bind _output_get (set `self.Health` 5)))

(fn `UserConstructionScript`)