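; Drivable car pawn with health, death and respawn, plus engine sound, HUD and a velocity-doubling boost.
; Axis inputs feed throttle and steering, with full throttle forced while unpossessed.
; Shots reduce health stored per car index in MyGameInstance; depleted health, or cooldown-limited flip and spin checks on Tick, trigger Kill.
; Kill spawns an explosion and shattering destructible, then teleports the same car above its death spot and restores health.
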(event `Shot`
  (params (VehicleID :type Integer))
  (`/Engine/EditorBlueprintResources/StandardMacros.DecrementInt` (stale `InitHealth` _currenthp)
    (:`  `
      (bind _currenthp (`self.SetHealth` 1))
      (set `self.healthPercentage` (/ (`KismetMathLibrary.Conv_IntToDouble` _currenthp) (`KismetMathLibrary.Conv_IntToDouble` (`self.maxHealth`))))
      (`/Engine/EditorBlueprintResources/StandardMacros.CompareInt` _currenthp
        (:`==`
          _)
        (:`<`
          _))
      (`self.Kill`))))

(event `Kill`
  (bind _returnvalue (`self.K2_GetActorLocation`))
  (bind _mesh (`self.Mesh`))
  ;[1 1 1] Death
  (`/Game/Turret_AI/TargetCom.SetisDead` (`self.TargetCom`) true)
  (`GameplayStatics.SpawnEmitterAtLocation` "/Game/StarterContent/Particles/P_Explosion.P_Explosion" _returnvalue)
  (`GameplayStatics.PlaySoundAtLocation` "/Game/StarterContent/Audio/Explosion02.Explosion02" _returnvalue)
  (bind _returnvalue_2 (`|SpawnActorFromClass` "/Game/Destruction/destructibleCube.destructibleCube_C" (`KismetMathLibrary.Conv_VectorToTransform` _returnvalue) "AlwaysSpawn" "OverrideRootScale"))
  (`DestructibleComponent.ApplyRadiusDamage` (`/Game/Destruction/destructibleCube.Destructible` _returnvalue_2) 10000.0 _returnvalue 1000.0 1000.0 true)
  ;[1 1 1] Respawning
  (set `self.spawnLocation` (`SceneComponent.K2_GetComponentLocation` _mesh))
  (set `self.spawnRotation` (`KismetMathLibrary.MakeRotator` 0.0 (.pitch (`SceneComponent.K2_GetComponentRotation` _mesh)) (.yaw (`SceneComponent.K2_GetComponentRotation` _mesh))))
  (`PrimitiveComponent.SetPhysicsAngularVelocity` _mesh (0.0 0.0 0.0) false "None")
  (`PrimitiveComponent.SetPhysicsLinearVelocity` _mesh (0.0 0.0 0.0) false "None")
  (`SceneComponent.K2_SetWorldRotation` _mesh (`self.spawnRotation`) false true)
  (`SceneComponent.K2_SetWorldLocation` _mesh (+ (`self.spawnLocation`) (0.0 0.0 500.0)) false true)
  (`/Game/Turret_AI/TargetCom.SetisDead` (`self.TargetCom`) false)
  (bind _currenthp (`self.SetHealth` (* (- (`self.maxHealth`) 1) -1)))
  (set `self.currentHealth` _currenthp)
  (set `self.healthPercentage` 1.0))

(event `self.ReceiveBeginPlay`
  (bind _mesh (`self.Mesh`))
  (`GameplayStatics.SpawnSoundAttached` "/Game/Sounds/Engine.Engine" (`self.Mesh`) "None" (0.0 0.0 0.0) (struct) "KeepRelativeOffset" false 0.01 0.5)
  (bind _returnvalue (`|CreateWidget` "/Game/GUI/MainMenu.MainMenu_C"))
  (set `self.Main Menu Reference` _returnvalue)
  (bind _returnvalue_2 (`|CreateWidget` "/Game/GUI/HUD.HUD_C"))
  (bind _output_get (set `self.HUD Reference` _returnvalue_2))
  (`UserWidget.AddToViewport` _output_get 0)
  (set `self.spawnLocation` (`SceneComponent.K2_GetComponentLocation` _mesh))
  (set `self.spawnRotation` (`SceneComponent.K2_GetComponentRotation` _mesh)))

(event `InitHealth`
  (bind _currenthp (`self.GetHealth`)))

(event `InputAxis|Forward`
  (params (AxisValue :type "Float (single-precision)"))
  ;[1 1 1] Driving
  (set `self.ThrottleVal` AxisValue))

(event `self.ReceiveTick`
  (params (DeltaSeconds :type "Float (single-precision)"))
  ;[1 1 1] Driving
  (set `self.lastDeath` (+ DeltaSeconds (`self.lastDeath`)))
  (`self.CheckRotation`)
  (`self.CheckVelocity`)
  (if (not (`self.isPossessed`))
    (set `self.ThrottleVal` 1.0))
  (`WheeledVehicleMovementComponent.SetThrottleInput` (`self.VehicleMovement`) (`self.ThrottleVal`)))

(event `InputAxis|Right`
  (params (AxisValue :type "Float (single-precision)"))
  ;[1 1 1] Driving
  (`WheeledVehicleMovementComponent.SetSteeringInput` (`self.VehicleMovement`) AxisValue))

(event `CheckRotation`
  (bind _returnvalue (`KismetMathLibrary.Abs` (.roll (`SceneComponent.K2_GetComponentRotation` (`self.Mesh`)))))
  ;[1 1 1] Death Logic
  (`/Engine/EditorBlueprintResources/StandardMacros.CompareFloat` _returnvalue 120.0
    (:`>`
      (`KismetSystemLibrary.Delay` 0.5)
      (`/Engine/EditorBlueprintResources/StandardMacros.CompareFloat` _returnvalue 120.0
        (:`>`
          (`self.DeathCheck`))))))

(event `CheckVelocity`
  ;[1 1 1] Death Logic
  (bind _returnvalue (`PrimitiveComponent.GetPhysicsAngularVelocity` (`self.Mesh`) "None"))
  (`/Engine/EditorBlueprintResources/StandardMacros.CompareFloat` (+ (`KismetMathLibrary.Abs` (.x _returnvalue)) (`KismetMathLibrary.Abs` (.y _returnvalue))) 900.0
    (:`>`
      (`self.DeathCheck`))))

(event `DeathCheck`
  ;[1 1 1] Death Logic
  (`/Engine/EditorBlueprintResources/StandardMacros.CompareFloat` (`self.lastDeath`) 2.0
    (:`>`
      (set `self.lastDeath` 0.0)
      (`self.Kill`))))

(fn `GetChosenCharacter`
  (set `self.characterChosen` (`/Game/GUI/MainMenu.CharacterChoice` (`self.Main Menu Reference`))))

(fn `GetHealth`
  (returns (currentHP :type Integer))
  (bind _asmy_game_instance (cast `/Game/GUI/MyGameInstance` (`GameplayStatics.GetGameInstance`))
    (:`then`
      _)
    (:`CastFailed`
      _))
  (return (`KismetArrayLibrary.Array_Get` (`/Game/GUI/MyGameInstance.Healths` _asmy_game_instance) (`self.ourIndex`))))

(fn `PlayerBoostPad`
  (bind _mesh (`self.Mesh`))
  (bind _returnvalue (`PrimitiveComponent.GetPhysicsLinearVelocity` _mesh "None"))
  (`PrimitiveComponent.SetPhysicsLinearVelocity` _mesh (* _returnvalue 2.0) false "None"))

(fn `SetHealth`
  (params (HealthDelta :type Integer))
  (returns (currentHP :type Integer))
  (bind _ourindex (`self.ourIndex`))
  (bind _maxhealth (`self.maxHealth`))
  (bind _asmy_game_instance (cast `/Game/GUI/MyGameInstance` (`GameplayStatics.GetGameInstance`))
    (:`then`
      _)
    (:`CastFailed`
      _))
  (bind _returnvalue (- (`KismetArrayLibrary.Array_Get` (`/Game/GUI/MyGameInstance.Healths` _asmy_game_instance) _ourindex) HealthDelta))
  (`/Engine/EditorBlueprintResources/StandardMacros.CompareInt` _returnvalue _maxhealth
    (:`>`
      _)
    (:`==`
      _)
    (:`<`
      (bind _healths (`/Game/GUI/MyGameInstance.Healths` _asmy_game_instance))
      (`KismetArrayLibrary.Array_Set` _healths _ourindex _returnvalue)
      (return _returnvalue)))
  (`KismetArrayLibrary.Array_Set` _healths _ourindex _maxhealth)
  (return _maxhealth))

(fn `UserConstructionScript`)